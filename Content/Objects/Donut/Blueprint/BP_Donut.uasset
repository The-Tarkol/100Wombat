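; BP_Donut is a donut pickup that the player character eats on contact.
; Tick spins the actor around its yaw axis at RotationSpeed.
; When BP_ThirdPersonCharacter overlaps the Sphere, it disables the sphere's collision and calls EatDonut on the character.
; The donut then destroys itself after a delay equal to the character's MunchTime.
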(event `self.ReceiveActorBeginOverlap`
  (params (OtherActor :type "Actor Object Reference")))

(event `self.ReceiveTick`
  (params (DeltaSeconds :type "Float (single-precision)"))
  (`self.K2_AddActorLocalRotation` (`KismetMathLibrary.MakeRotator` 0.0 0.0 (* DeltaSeconds (`self.RotationSpeed`)))))

(event `self.Sphere.OnComponentBeginOverlap`
  (params (OverlappedComponent :type "PrimitiveComponent Object Reference") (OtherActor :type "Actor Object Reference") (OtherComp :type "PrimitiveComponent Object Reference") (OtherBodyIndex :type Integer) (bFromSweep :type Boolean) (SweepResult :type "HitResult Structure (by ref)"))
  (bind _asbp_third_person_character (cast `/Game/ThirdPerson/Blueprints/BP_ThirdPersonCharacter` OtherActor))
  (`PrimitiveComponent.SetCollisionEnabled` (`self.Sphere`) "NoCollision")
  (`/Game/ThirdPerson/Blueprints/BP_ThirdPersonCharacter.EatDonut` _asbp_third_person_character)
  (`KismetSystemLibrary.Delay` (`/Game/ThirdPerson/Blueprints/BP_ThirdPersonCharacter.MunchTime` _asbp_third_person_character))
  (`self.K2_DestroyActor`))

(fn `UserConstructionScript`)